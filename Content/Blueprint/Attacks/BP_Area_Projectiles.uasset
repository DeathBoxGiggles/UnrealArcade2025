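; BP_Area_Projectiles is an area attack actor that sends four spheres outward from its origin in a cross pattern.
; On BeginPlay, a Sequence starts four timelines, each lerping one sphere's relative location 1000 units along positive or negative X or Y, without sweep.
; The first timeline's update also triggers a short Delay, after which the actor destroys itself.
; No hit or damage logic is in these graphs.
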(event `self.ReceiveBeginPlay`
  (`|ExecutionSequence`
    (:`then_0`
      (bind (_direction _newtrack_0) (`Timeline|Timeline` :!via `PlayFromStart`)
        (:`Update`
          (`SceneComponent.K2_SetRelativeLocation` (`self.Sphere`) (`KismetMathLibrary.VLerp` (0.0 0.0 0.0) (1000.0 0.0 0.0) _newtrack_0) false false)
          (`KismetSystemLibrary.Delay` 1.01)
          (`self.K2_DestroyActor`))))
    (:`then_1`
      (bind (_direction_2 _newtrack_0_2) (`Timeline|Timeline_0` :!via `PlayFromStart`)
        (:`Update`
          (`SceneComponent.K2_SetRelativeLocation` (`self.Sphere1`) (`KismetMathLibrary.VLerp` (0.0 0.0 0.0) (-1000.0 0.0 0.0) _newtrack_0_2) false false))))
    (:`then_2`
      (bind (_direction_3 _newtrack_0_3) (`Timeline|Timeline_1` :!via `PlayFromStart`)
        (:`Update`
          (`SceneComponent.K2_SetRelativeLocation` (`self.Sphere2`) (`KismetMathLibrary.VLerp` (0.0 0.0 0.0) (0.0 1000.0 0.0) _newtrack_0_3) false false))))
    (:`then_3`
      (bind (_direction_4 _newtrack_0_4) (`Timeline|Timeline_2` :!via `PlayFromStart`)
        (:`Update`
          (`SceneComponent.K2_SetRelativeLocation` (`self.Sphere3`) (`KismetMathLibrary.VLerp` (0.0 0.0 0.0) (0.0 -1000.0 0.0) _newtrack_0_4) false false))))))

(fn `UserConstructionScript`)