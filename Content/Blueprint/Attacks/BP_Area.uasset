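; BP_Area is an expanding area attack that detects the player character.
; On BeginPlay a timeline scales its mesh wide in X and Y while Z stays fixed.
; Delays chained from the timeline's update disable the Cylinder's collision, then destroy the actor shortly after.
; Cylinder overlaps send begin and end messages to the player, with a Once flag guarding repeated begins until the tick after overlap ends.
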(event `self.ReceiveBeginPlay`
  (bind (_direction _newtrack_0) (`Timeline|Timeline` :!via `PlayFromStart`)
    (:`Update`
      (`SceneComponent.SetWorldScale3D` (`self.StaticMesh`) (`KismetMathLibrary.VLerp` (1.0 1.0 1.0) (20.0 20.0 1.0) _newtrack_0))
      (`KismetSystemLibrary.Delay` 2.0)
      (`PrimitiveComponent.SetCollisionEnabled` (`self.Cylinder`) "NoCollision")
      (`KismetSystemLibrary.Delay` 0.1)
      (`self.K2_DestroyActor`))))

(event `self.Cylinder.OnComponentBeginOverlap`
  (params (OverlappedComponent :type "PrimitiveComponent Object Reference") (OtherActor :type "Actor Object Reference") (OtherComp :type "PrimitiveComponent Object Reference") (OtherBodyIndex :type Integer) (bFromSweep :type Boolean) (SweepResult :type "HitResult Structure (by ref)"))
  (if (== OtherActor (`GameplayStatics.GetPlayerCharacter` 0))
    (if (not (`self.Once`))
      (set `self.Once` true)
      (message `/Game/Blueprint/Attacks/BPI_Player.IsOverlapping` (`GameplayStatics.GetPlayerCharacter` 0)))))

(event `self.Cylinder.OnComponentEndOverlap`
  (params (OverlappedComponent :type "PrimitiveComponent Object Reference") (OtherActor :type "Actor Object Reference") (OtherComp :type "PrimitiveComponent Object Reference") (OtherBodyIndex :type Integer))
  (if (== OtherActor (`GameplayStatics.GetPlayerCharacter` 0))
    (message `/Game/Blueprint/Attacks/BPI_Player.EndOverlap` (`GameplayStatics.GetPlayerCharacter` 0))
    (`KismetSystemLibrary.DelayUntilNextTick`)
    (set `self.Once` false)))

(fn `UserConstructionScript`)