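; Base player Blueprint for an arcade-style game, handling movement, shooting and an area ability through Enhanced Input.
; Movement follows world axes and snaps control rotation to cardinal yaws.
; Shooting box-traces from an arrow component and damages the hit actor, with debug drawing and printing.
; The area input spawns BP_Area on a two-second cooldown, or BP_Area_Projectiles while an event-set overlap flag is true; pause quits the game.
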(event `self.ReceiveBeginPlay`
  (`EnhancedInputSubsystemInterface.AddMappingContext` (pcsubsystem `EnhancedInputLocalPlayerSubsystem` (`GameplayStatics.GetPlayerController` 0)) "/Game/Blueprint/Input/ArcadeActionMapping.ArcadeActionMapping" 0 (struct)))

(event `EnhancedInput|/Game/Blueprint/Input/IA_Move`
  (params (ActionValue :type "Vector2D Structure") (ElapsedSeconds :type "Float (double-precision)") (TriggeredSeconds :type "Float (double-precision)") (InputAction :type "InputAction Object Reference" :default "/Game/Blueprint/Input/IA_Move.IA_Move"))
  (:`Triggered`
    (`self.Move` ActionValue_X ActionValue_Y)))

(event `EnhancedInput|/Game/Blueprint/Input/IA_Pause`
  (params (ActionValue :type Boolean) (ElapsedSeconds :type "Float (double-precision)") (TriggeredSeconds :type "Float (double-precision)") (InputAction :type "InputAction Object Reference" :default "/Game/Blueprint/Input/IA_Pause.IA_Pause"))
  (:`Triggered`
    (`KismetSystemLibrary.QuitGame` null "Quit")))

(event `EnhancedInput|/Game/Blueprint/Input/IA_Shoot`
  (params (ActionValue :type Boolean) (ElapsedSeconds :type "Float (double-precision)") (TriggeredSeconds :type "Float (double-precision)") (InputAction :type "InputAction Object Reference" :default "/Game/Blueprint/Input/IA_Shoot.IA_Shoot"))
  (bind _arrow1 (`self.Arrow1`))
  (bind _returnvalue (`SceneComponent.K2_GetComponentLocation` _arrow1))
  (:`Started`
    (bind _outhit (`KismetSystemLibrary.BoxTraceSingle` :`Start` _returnvalue :`End` (+ _returnvalue (* (`KismetMathLibrary.GetForwardVector` (`SceneComponent.K2_GetComponentRotation` _arrow1)) 1000000.0)) :`HalfSize` (100.0 100.0 100.0) :`TraceChannel` "TraceTypeQuery1" :`DrawDebugType` "Persistent"))
    (bind (_bblockinghit _binitialoverlap _time _distance _location _impactpoint _normal _impactnormal _physmat _hitactor) (`GameplayStatics.BreakHitResult` _outhit))
    (`KismetSystemLibrary.PrintString` (`KismetSystemLibrary.GetDisplayName` _hitactor))
    (`GameplayStatics.ApplyDamage` _hitactor 100.0)))

(event `EnhancedInput|/Game/Blueprint/Input/IA_Area`
  (params (ActionValue :type Boolean) (ElapsedSeconds :type "Float (double-precision)") (TriggeredSeconds :type "Float (double-precision)") (InputAction :type "InputAction Object Reference" :default "/Game/Blueprint/Input/IA_Area.IA_Area"))
  (:`Started`
    (if (`self.Overlapping`)
      (`|SpawnActorFromClass` "/Game/Blueprint/Attacks/BP_Area_Projectiles.BP_Area_Projectiles_C" (`KismetMathLibrary.MakeTransform` (+ (`self.K2_GetActorLocation`) (0.0 0.0 0.0))) "Undefined" "MultiplyWithRoot" null null)
      (elif (not (`self.Area Fired`))
        (set `self.Area Fired` true)
        (`|SpawnActorFromClass` "/Game/Blueprint/Attacks/BP_Area.BP_Area_C" (`KismetMathLibrary.MakeTransform` (+ (`self.K2_GetActorLocation`) (0.0 0.0 -50.0))) "Undefined" "MultiplyWithRoot" null null)
        (`KismetSystemLibrary.Delay` 2.01)
        (set `self.Area Fired` false)))))

(event `/Game/Blueprint/Attacks/BPI_Player.IsOverlapping`
  (set `self.Overlapping` true))

(event `/Game/Blueprint/Attacks/BPI_Player.EndOverlap`
  (set `self.Overlapping` false))

(fn `Move`
  (params (`Axis X` :type "Float (double-precision)") (`Axis Y` :type "Float (double-precision)"))
  (`self.AddMovementInput` (1.0 0.0 0.0) `Axis X`)
  (`self.AddMovementInput` (0.0 1.0 0.0) `Axis Y`)
  (`Controller.SetControlRotation` (`GameplayStatics.GetPlayerController` 0) (`KismetMathLibrary.MakeRotator` 0.0 0.0 (+ (select `bool` (`KismetMathLibrary.InRange_FloatFloat` `Axis Y` -1.0 -0.01) :`true` -90.0 :!type "Float (single-precision)") (select `bool` (`KismetMathLibrary.InRange_FloatFloat` `Axis Y` 0.01) :`true` 90.0 :!type "Float (single-precision)") (select `bool` (`KismetMathLibrary.InRange_FloatFloat` `Axis X` -1.0 -0.01) :`true` 180.0 :!type "Float (single-precision)")))))

(fn `UserConstructionScript`)